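; Desert biome editor tool that builds cliff walls by placing spline meshes along an editable spline in the Construction Script.
; The spline is split into evenly stretched sections, or one if Single, with cliff meshes chosen by type, seeded random or sequence.
; Sections support flipping, bending, loop shifting, material overrides, collision and push-out via mesh offsets or cached point scaling.
; Optional single or spline-distributed decals have per-index pitch tweaks and debug labels.
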(event EventBeginPlay)

(event Collision|EventActorBeginOverlap
  (params (OtherActor :type Actor%20Object%20Reference)))

(event EventTick
  (params (DeltaSeconds :type Float%20%28single-precision%29)))

(fn ConstructionScript
  (bind (_start_position _end_possition _start_tangent1 _end_tangent) (CallFunction|GetSplineMeshPositionandTangents))
  (bind _spline (Variables|Default|GetSpline))
  (bind _push_out_meshes (Variables|Default|GetPush%20Out%20Meshes))
  (bind _spline_2 (Variables|Default|GetSpline))
  (bind _returnvalue (Spline|GetSplineLength _spline))
  (bind _returnvalue_2 (* _push_out_meshes 7.5e+02))
  (bind _returnvalue_3 (Math|Vector2D|MakeVector2D _returnvalue_2 0.0))
  ;[1 1 1] push out setup
  (Variables|Default|SetPush%20Out%20Spline%20Internal (Variables|Default|GetPush%20Out%20Spline))
  (Variables|Default|SetStart%20Offset%20Internal _returnvalue_3)
  (Variables|Default|SetEnd%20Offset%20Internal _returnvalue_3)
  ;[1 1 1] Seed and Spline update
  (Math|Random|SetRandomStreamSeed (Variables|Default|GetRandomStream) (Variables|Default|GetRandom%20Seed))
  (Spline|SetClosedLoop _spline_2 (Variables|Default|GetIs%20Closed%20Loop) true)
  (Spline|UpdateSpline _spline_2)
  ;[1 1 1] offset setup
  (bind _output_get (Variables|Default|SetOffset_Internal (* (Variables|Default|GetOffset) 7.5e+02)))
  (Variables|Default|Setshift _output_get)
  (Utilities|FlowControl|Sequence ; sequence
    (:then_0
      ;[1 1 1] Decals
      (CallFunction|AddSimpleDecal))
    (:then_1
      (CallFunction|AddMultiDecal))
    (:then_2
      (if (Variables|Default|GetCache%20Spline%20Points)
        (for _index (range 0 (Spline|GetNumberOfSplinePoints (Variables|Default|GetSpline))) ; start loop
          (Variables|Default|SetSpline%20Point%20Index _index)
          (Utilities|Array|Add (Variables|Default|GetSplinePointLocationArray) (/ (Spline|GetLocationatSplinePoint (Variables|Default|GetSpline) _index "Local") (Variables|Default|GetPush%20Out%20Spline%20Internal%20Previous))))))
    (:then_3
      (if (Variables|Default|GetEnable%20Spline%20Point%20Setting)
        (for _index_2 (range 0 (Spline|GetNumberOfSplinePoints (Variables|Default|GetSpline))) ; start loop
          (Spline|SetLocationatSplinePoint (Variables|Default|GetSpline) _index_2 (* (/ (Utilities|Array|Get(acopy) (Variables|Default|GetSplinePointLocationArray) _index_2) (Variables|Default|GetPush%20Out%20Spline%20Internal%20Previous)) (Variables|Default|GetPush%20Out%20Spline%20Internal)) "Local" true))
        (else
          (Variables|Default|SetPush%20Out%20Spline%20Internal%20Previous (Variables|Default|GetPush%20Out%20Spline%20Internal)))))
    (:then_4
      (if (Variables|Default|GetSingle)
        (Variables|Default|SetIndex_A 0)
        (bind _output_get_2 (Variables|Default|SetSplineLength _returnvalue))
        (Variables|Default|SetCorrected%20Section%20Length _output_get_2)
        (bind _output_get_3 (Variables|Default|SetIs%20Closed%20Loop false))
        (Spline|SetClosedLoop (Variables|Default|GetSpline) _output_get_3 true)
        (else
          ;[1 1 1] get spline length and set amount of meshes
          (bind _output_get_4 (Variables|Default|SetSplineLength _returnvalue))
          (Variables|Default|SetIndex_A (Math|Float|Truncate (/ _output_get_4 (Variables|Default|GetSectionLength))))
          (Variables|Default|SetCorrected%20Section%20Length (/ (Spline|GetSplineLength (Variables|Default|GetSpline)) (Math|Conversions|ToFloat(Integer) (+ (Variables|Default|GetIndex_A) 1)))))))
    (:then_5
      (Variables|Default|SetMesh%20Sequence%20Number (Variables|Default|GetMesh%20Sequence%20Offset))
      (for _index_3 (range 0 (Variables|Default|GetIndex_A)) ; start loop
        (if (Variables|Default|GetSequence%20Meshes)
          (bind _result (Math|Integer|IncrementInt (Variables|Default|GetMesh%20Sequence%20Number))
            (:%20%20
              (if (Math|Integer|InRange(Integer) _result 0 2)
                _
                (else
                  (Variables|Default|SetMesh%20Sequence%20Number 0))))))
        (Variables|Default|SetSectionLength_Current (* _index_3 (Variables|Default|GetCorrected%20Section%20Length)))
        (if (Variables|Default|GetFar%20Shadow)
          (bind _returnvalue_4 (AddComponent|AddSplineMeshComponent false))
          (Variables|Default|SetCurrent%20Spline%20Mesh _returnvalue_4)
          (else
            (bind _returnvalue_5 (AddComponent|AddSplineMeshComponent false))
            (Variables|Default|SetCurrent%20Spline%20Mesh _returnvalue_5)))
        (Class|PrimitiveComponent|SetCullDistance (Variables|Default|GetCurrent%20Spline%20Mesh) (Variables|Default|GetCull%20Distance))
        (Components|StaticMesh|SetStaticMesh (Variables|Default|GetCurrent%20Spline%20Mesh) (CallFunction|GetSplineStaticMesh))
        (SplineMesh|SetStartandEnd (Variables|Default|GetCurrent%20Spline%20Mesh) _start_position _start_tangent1 _end_possition _end_tangent true :!class /Script/Engine.SplineMeshComponent)
        (Variables|Material|SetOriginal%20Material (Rendering|Material|GetMaterial (Variables|Default|GetCurrent%20Spline%20Mesh) 0))
        (Rendering|SetReceivesDecals (Variables|Default|GetCurrent%20Spline%20Mesh) (Variables|Default|GetReceives%20Decals))
        (Rendering|Material|SetMaterial (Variables|Default|GetCurrent%20Spline%20Mesh) 0 (Variables|Material|GetOverride%20Material))
        (if (> (Utilities|Array|Length (Rendering|Material|GetMaterials (Variables|Default|GetCurrent%20Spline%20Mesh))) 1)
          (Rendering|Material|SetMaterial (Variables|Default|GetCurrent%20Spline%20Mesh) 1 (Variables|Material|Get2nd%20Override%20Material))
          (if (> (Utilities|Array|Length (Rendering|Material|GetMaterials (Variables|Default|GetCurrent%20Spline%20Mesh))) 2)
            (Rendering|Material|SetMaterial (Variables|Default|GetCurrent%20Spline%20Mesh) 2 (Variables|Material|Get3rd%20Override%20Material))))
        (SplineMesh|SetStartOffset (Variables|Default|GetCurrent%20Spline%20Mesh) (Variables|Default|GetStart%20Offset%20Internal) true)
        (SplineMesh|SetEndOffset (Variables|Default|GetCurrent%20Spline%20Mesh) (Variables|Default|GetEnd%20Offset%20Internal) true)
        (Utilities|Array|Add (Variables|Default|GetSplineMeshArray) (Variables|Default|GetCurrent%20Spline%20Mesh))))
    (:then_6
      ;[1 1 1] Handle collision
      (if (Variables|Default|GetEnable%20Collision)
        (for _array_element (Variables|Default|GetSplineMeshArray)
          (Collision|SetCollisionEnabled _array_element "QueryAndPhysics"))))
    (:then_7
      ;[1 1 1] Resize arrays
      (Utilities|Array|Resize (Variables|Default|GetSplinePointLocationArray) (Variables|Default|GetSpline%20Point%20Index))
      (Utilities|Array|Resize (Variables|Default|GetSplineMeshArray) (* (Variables|Default|GetIndex_A) 2)))))

(fn GetSplineMeshStartEndPositionandTangents
  (params (Spline%20Section%20Size :type Float%20%28double-precision%29) (Spline%20Point :type Integer))
  (bind _spline (Variables|Default|GetSpline))
  (Variables|Default|SetMax%20Spline%20Length (Spline|GetSplineLength (Variables|Default|GetSpline)))
  (Variables|Default|SetSplinePoint%20Temp Spline%20Point)
  (Spline|UpdateSpline (Variables|Default|GetSpline))
  (Variables|Default|SetSplineDistance%20Temp Spline%20Section%20Size)
  (return (* (Utilities|Select :Index (Variables|Default|GetTangentType) :NewEnumerator0 (Math|Vector|MakeVector 0.0 0.0 0.0) :NewEnumerator1 (Math|Vector|ClampVectorSize (Spline|GetTangentatDistanceAlongSpline (Variables|Default|GetSpline) (select (Variables|Default|GetFlip%20Mesh) (select (>= (+ (* (Variables|Default|GetSplinePoint%20Temp) (- (Variables|Default|GetSplineDistance%20Temp) (Variables|Advanced:GapOffsets|GetOffset%20Start%20Position))) (Variables|Default|GetOffset_Internal)) (Variables|Default|GetMax%20Spline%20Length)) (Math|Float|%(Float) (+ (* (Variables|Default|GetSplinePoint%20Temp) (- (Variables|Default|GetSplineDistance%20Temp) (Variables|Advanced:GapOffsets|GetOffset%20Start%20Tangent))) (Variables|Default|GetOffset_Internal)) (Variables|Default|GetMax%20Spline%20Length)) (+ (* (Variables|Default|GetSplinePoint%20Temp) (- (Variables|Default|GetSplineDistance%20Temp) (Variables|Advanced:GapOffsets|GetOffset%20Start%20Tangent))) (Variables|Default|GetOffset_Internal))) (select (>= (+ (* (+ (Variables|Default|GetSplinePoint%20Temp) 1) (+ (Variables|Default|GetSplineDistance%20Temp) (Variables|Advanced:GapOffsets|GetOffset%20End%20Pos))) (Variables|Default|GetOffset_Internal)) (Variables|Default|GetMax%20Spline%20Length)) (Math|Float|%(Float) (+ (* (+ (Variables|Default|GetSplinePoint%20Temp) 1) (+ (Variables|Default|GetSplineDistance%20Temp) (Variables|Advanced:GapOffsets|GetOffset%20End%20Tangent))) (Variables|Default|GetOffset_Internal)) (Variables|Default|GetMax%20Spline%20Length)) (+ (* (+ (Variables|Default|GetSplinePoint%20Temp) 1) (+ (Variables|Default|GetSplineDistance%20Temp) (Variables|Advanced:GapOffsets|GetOffset%20End%20Tangent))) (Variables|Default|GetOffset_Internal)))) "Local") 0.0 (Variables|Default|GetSplineDistance%20Temp)) :NewEnumerator2 (Spline|GetDirectionatDistanceAlongSpline (Variables|Default|GetSpline) (select (Variables|Default|GetFlip%20Mesh) (select (>= (+ (* (Variables|Default|GetSplinePoint%20Temp) (- (Variables|Default|GetSplineDistance%20Temp) (Variables|Advanced:GapOffsets|GetOffset%20Start%20Position))) (Variables|Default|GetOffset_Internal)) (Variables|Default|GetMax%20Spline%20Length)) (Math|Float|%(Float) (+ (* (Variables|Default|GetSplinePoint%20Temp) (- (Variables|Default|GetSplineDistance%20Temp) (Variables|Advanced:GapOffsets|GetOffset%20Start%20Tangent))) (Variables|Default|GetOffset_Internal)) (Variables|Default|GetMax%20Spline%20Length)) (+ (* (Variables|Default|GetSplinePoint%20Temp) (- (Variables|Default|GetSplineDistance%20Temp) (Variables|Advanced:GapOffsets|GetOffset%20Start%20Tangent))) (Variables|Default|GetOffset_Internal))) (select (>= (+ (* (+ (Variables|Default|GetSplinePoint%20Temp) 1) (+ (Variables|Default|GetSplineDistance%20Temp) (Variables|Advanced:GapOffsets|GetOffset%20End%20Pos))) (Variables|Default|GetOffset_Internal)) (Variables|Default|GetMax%20Spline%20Length)) (Math|Float|%(Float) (+ (* (+ (Variables|Default|GetSplinePoint%20Temp) 1) (+ (Variables|Default|GetSplineDistance%20Temp) (Variables|Advanced:GapOffsets|GetOffset%20End%20Tangent))) (Variables|Default|GetOffset_Internal)) (Variables|Default|GetMax%20Spline%20Length)) (+ (* (+ (Variables|Default|GetSplinePoint%20Temp) 1) (+ (Variables|Default|GetSplineDistance%20Temp) (Variables|Advanced:GapOffsets|GetOffset%20End%20Tangent))) (Variables|Default|GetOffset_Internal)))) "Local") :NewEnumerator3 (Math|Rotator|GetRotationXVector (Spline|GetRotationatDistanceAlongSpline (Variables|Default|GetSpline) (select (Variables|Default|GetFlip%20Mesh) (select (>= (+ (* (Variables|Default|GetSplinePoint%20Temp) (- (Variables|Default|GetSplineDistance%20Temp) (Variables|Advanced:GapOffsets|GetOffset%20Start%20Position))) (Variables|Default|GetOffset_Internal)) (Variables|Default|GetMax%20Spline%20Length)) (Math|Float|%(Float) (+ (* (Variables|Default|GetSplinePoint%20Temp) (- (Variables|Default|GetSplineDistance%20Temp) (Variables|Advanced:GapOffsets|GetOffset%20Start%20Tangent))) (Variables|Default|GetOffset_Internal)) (Variables|Default|GetMax%20Spline%20Length)) (+ (* (Variables|Default|GetSplinePoint%20Temp) (- (Variables|Default|GetSplineDistance%20Temp) (Variables|Advanced:GapOffsets|GetOffset%20Start%20Tangent))) (Variables|Default|GetOffset_Internal))) (select (>= (+ (* (+ (Variables|Default|GetSplinePoint%20Temp) 1) (+ (Variables|Default|GetSplineDistance%20Temp) (Variables|Advanced:GapOffsets|GetOffset%20End%20Pos))) (Variables|Default|GetOffset_Internal)) (Variables|Default|GetMax%20Spline%20Length)) (Math|Float|%(Float) (+ (* (+ (Variables|Default|GetSplinePoint%20Temp) 1) (+ (Variables|Default|GetSplineDistance%20Temp) (Variables|Advanced:GapOffsets|GetOffset%20End%20Tangent))) (Variables|Default|GetOffset_Internal)) (Variables|Default|GetMax%20Spline%20Length)) (+ (* (+ (Variables|Default|GetSplinePoint%20Temp) 1) (+ (Variables|Default|GetSplineDistance%20Temp) (Variables|Advanced:GapOffsets|GetOffset%20End%20Tangent))) (Variables|Default|GetOffset_Internal)))) "Local"))) (Variables|Advanced:GapOffsets|GetTangent%20Scale)) (* (Utilities|Select :Index (Variables|Default|GetTangentType) :NewEnumerator0 "0, 0, 0" :NewEnumerator1 (Math|Vector|ClampVectorSize (Spline|GetTangentatDistanceAlongSpline _spline (select (Variables|Default|GetFlip%20Mesh) (select (>= (+ (* (+ (Variables|Default|GetSplinePoint%20Temp) 1) (+ (Variables|Default|GetSplineDistance%20Temp) (Variables|Advanced:GapOffsets|GetOffset%20End%20Pos))) (Variables|Default|GetOffset_Internal)) (Variables|Default|GetMax%20Spline%20Length)) (Math|Float|%(Float) (+ (* (+ (Variables|Default|GetSplinePoint%20Temp) 1) (+ (Variables|Default|GetSplineDistance%20Temp) (Variables|Advanced:GapOffsets|GetOffset%20End%20Tangent))) (Variables|Default|GetOffset_Internal)) (Variables|Default|GetMax%20Spline%20Length)) (+ (* (+ (Variables|Default|GetSplinePoint%20Temp) 1) (+ (Variables|Default|GetSplineDistance%20Temp) (Variables|Advanced:GapOffsets|GetOffset%20End%20Tangent))) (Variables|Default|GetOffset_Internal))) (select (>= (+ (* (Variables|Default|GetSplinePoint%20Temp) (- (Variables|Default|GetSplineDistance%20Temp) (Variables|Advanced:GapOffsets|GetOffset%20Start%20Position))) (Variables|Default|GetOffset_Internal)) (Variables|Default|GetMax%20Spline%20Length)) (Math|Float|%(Float) (+ (* (Variables|Default|GetSplinePoint%20Temp) (- (Variables|Default|GetSplineDistance%20Temp) (Variables|Advanced:GapOffsets|GetOffset%20Start%20Tangent))) (Variables|Default|GetOffset_Internal)) (Variables|Default|GetMax%20Spline%20Length)) (+ (* (Variables|Default|GetSplinePoint%20Temp) (- (Variables|Default|GetSplineDistance%20Temp) (Variables|Advanced:GapOffsets|GetOffset%20Start%20Tangent))) (Variables|Default|GetOffset_Internal)))) "Local") 0.0 (Variables|Default|GetSplineDistance%20Temp)) :NewEnumerator2 (Spline|GetDirectionatDistanceAlongSpline (Variables|Default|GetSpline) (select (Variables|Default|GetFlip%20Mesh) (select (>= (+ (* (+ (Variables|Default|GetSplinePoint%20Temp) 1) (+ (Variables|Default|GetSplineDistance%20Temp) (Variables|Advanced:GapOffsets|GetOffset%20End%20Pos))) (Variables|Default|GetOffset_Internal)) (Variables|Default|GetMax%20Spline%20Length)) (Math|Float|%(Float) (+ (* (+ (Variables|Default|GetSplinePoint%20Temp) 1) (+ (Variables|Default|GetSplineDistance%20Temp) (Variables|Advanced:GapOffsets|GetOffset%20End%20Tangent))) (Variables|Default|GetOffset_Internal)) (Variables|Default|GetMax%20Spline%20Length)) (+ (* (+ (Variables|Default|GetSplinePoint%20Temp) 1) (+ (Variables|Default|GetSplineDistance%20Temp) (Variables|Advanced:GapOffsets|GetOffset%20End%20Tangent))) (Variables|Default|GetOffset_Internal))) (select (>= (+ (* (Variables|Default|GetSplinePoint%20Temp) (- (Variables|Default|GetSplineDistance%20Temp) (Variables|Advanced:GapOffsets|GetOffset%20Start%20Position))) (Variables|Default|GetOffset_Internal)) (Variables|Default|GetMax%20Spline%20Length)) (Math|Float|%(Float) (+ (* (Variables|Default|GetSplinePoint%20Temp) (- (Variables|Default|GetSplineDistance%20Temp) (Variables|Advanced:GapOffsets|GetOffset%20Start%20Tangent))) (Variables|Default|GetOffset_Internal)) (Variables|Default|GetMax%20Spline%20Length)) (+ (* (Variables|Default|GetSplinePoint%20Temp) (- (Variables|Default|GetSplineDistance%20Temp) (Variables|Advanced:GapOffsets|GetOffset%20Start%20Tangent))) (Variables|Default|GetOffset_Internal)))) "Local") :NewEnumerator3 (Math|Rotator|GetRotationXVector (Spline|GetRotationatDistanceAlongSpline (Variables|Default|GetSpline) (select (Variables|Default|GetFlip%20Mesh) (select (>= (+ (* (+ (Variables|Default|GetSplinePoint%20Temp) 1) (+ (Variables|Default|GetSplineDistance%20Temp) (Variables|Advanced:GapOffsets|GetOffset%20End%20Pos))) (Variables|Default|GetOffset_Internal)) (Variables|Default|GetMax%20Spline%20Length)) (Math|Float|%(Float) (+ (* (+ (Variables|Default|GetSplinePoint%20Temp) 1) (+ (Variables|Default|GetSplineDistance%20Temp) (Variables|Advanced:GapOffsets|GetOffset%20End%20Tangent))) (Variables|Default|GetOffset_Internal)) (Variables|Default|GetMax%20Spline%20Length)) (+ (* (+ (Variables|Default|GetSplinePoint%20Temp) 1) (+ (Variables|Default|GetSplineDistance%20Temp) (Variables|Advanced:GapOffsets|GetOffset%20End%20Tangent))) (Variables|Default|GetOffset_Internal))) (select (>= (+ (* (Variables|Default|GetSplinePoint%20Temp) (- (Variables|Default|GetSplineDistance%20Temp) (Variables|Advanced:GapOffsets|GetOffset%20Start%20Position))) (Variables|Default|GetOffset_Internal)) (Variables|Default|GetMax%20Spline%20Length)) (Math|Float|%(Float) (+ (* (Variables|Default|GetSplinePoint%20Temp) (- (Variables|Default|GetSplineDistance%20Temp) (Variables|Advanced:GapOffsets|GetOffset%20Start%20Tangent))) (Variables|Default|GetOffset_Internal)) (Variables|Default|GetMax%20Spline%20Length)) (+ (* (Variables|Default|GetSplinePoint%20Temp) (- (Variables|Default|GetSplineDistance%20Temp) (Variables|Advanced:GapOffsets|GetOffset%20Start%20Tangent))) (Variables|Default|GetOffset_Internal)))) "Local"))) (Variables|Advanced:GapOffsets|GetTangent%20Scale)) (Spline|GetLocationatDistanceAlongSpline (Variables|Default|GetSpline) (select (Variables|Default|GetFlip%20Mesh) (select (>= (+ (* (Variables|Default|GetSplinePoint%20Temp) (- (Variables|Default|GetSplineDistance%20Temp) (Variables|Advanced:GapOffsets|GetOffset%20Start%20Position))) (Variables|Default|GetOffset_Internal)) (Variables|Default|GetMax%20Spline%20Length)) (Math|Float|%(Float) (+ (* (Variables|Default|GetSplinePoint%20Temp) (- (Variables|Default|GetSplineDistance%20Temp) (Variables|Advanced:GapOffsets|GetOffset%20Start%20Position))) (Variables|Default|GetOffset_Internal)) (Variables|Default|GetMax%20Spline%20Length)) (+ (* (Variables|Default|GetSplinePoint%20Temp) (- (Variables|Default|GetSplineDistance%20Temp) (Variables|Advanced:GapOffsets|GetOffset%20Start%20Position))) (Variables|Default|GetOffset_Internal))) (select (>= (+ (* (+ (Variables|Default|GetSplinePoint%20Temp) 1) (+ (Variables|Default|GetSplineDistance%20Temp) (Variables|Advanced:GapOffsets|GetOffset%20End%20Pos))) (Variables|Default|GetOffset_Internal)) (Variables|Default|GetMax%20Spline%20Length)) (Math|Float|%(Float) (+ (* (+ (Variables|Default|GetSplinePoint%20Temp) 1) (+ (Variables|Default|GetSplineDistance%20Temp) (Variables|Advanced:GapOffsets|GetOffset%20End%20Pos))) (Variables|Default|GetOffset_Internal)) (Variables|Default|GetMax%20Spline%20Length)) (+ (* (+ (Variables|Default|GetSplinePoint%20Temp) 1) (+ (Variables|Default|GetSplineDistance%20Temp) (Variables|Advanced:GapOffsets|GetOffset%20End%20Pos))) (Variables|Default|GetOffset_Internal)))) "Local") (Spline|GetLocationatDistanceAlongSpline _spline (select (Variables|Default|GetFlip%20Mesh) (select (>= (+ (* (+ (Variables|Default|GetSplinePoint%20Temp) 1) (+ (Variables|Default|GetSplineDistance%20Temp) (Variables|Advanced:GapOffsets|GetOffset%20End%20Pos))) (Variables|Default|GetOffset_Internal)) (Variables|Default|GetMax%20Spline%20Length)) (Math|Float|%(Float) (+ (* (+ (Variables|Default|GetSplinePoint%20Temp) 1) (+ (Variables|Default|GetSplineDistance%20Temp) (Variables|Advanced:GapOffsets|GetOffset%20End%20Pos))) (Variables|Default|GetOffset_Internal)) (Variables|Default|GetMax%20Spline%20Length)) (+ (* (+ (Variables|Default|GetSplinePoint%20Temp) 1) (+ (Variables|Default|GetSplineDistance%20Temp) (Variables|Advanced:GapOffsets|GetOffset%20End%20Pos))) (Variables|Default|GetOffset_Internal))) (select (>= (+ (* (Variables|Default|GetSplinePoint%20Temp) (- (Variables|Default|GetSplineDistance%20Temp) (Variables|Advanced:GapOffsets|GetOffset%20Start%20Position))) (Variables|Default|GetOffset_Internal)) (Variables|Default|GetMax%20Spline%20Length)) (Math|Float|%(Float) (+ (* (Variables|Default|GetSplinePoint%20Temp) (- (Variables|Default|GetSplineDistance%20Temp) (Variables|Advanced:GapOffsets|GetOffset%20Start%20Position))) (Variables|Default|GetOffset_Internal)) (Variables|Default|GetMax%20Spline%20Length)) (+ (* (Variables|Default|GetSplinePoint%20Temp) (- (Variables|Default|GetSplineDistance%20Temp) (Variables|Advanced:GapOffsets|GetOffset%20Start%20Position))) (Variables|Default|GetOffset_Internal)))) "Local")))

(fn GetDecalScale
  (bind _defaultsceneroot (Variables|Default|GetDefaultSceneRoot))
  (bind _decal_size (Variables|Decal|GetDecal%20Size))
  (bind _returnvalue (Transformation|GetWorldScale _defaultsceneroot))
  ;[1 1 1] Handle decal scale and orientation (Z swap)
  (return (Math|Vector|MakeVector (* (* _decal_size (.z _returnvalue)) (Variables|Decal|GetDecal%20Projection%20Depth)) (* _decal_size (.y _returnvalue)) (* (.x _returnvalue) _decal_size))))

(fn AddSimpleDecal
  (bind _defaultsceneroot (Variables|Default|GetDefaultSceneRoot))
  (bind _decal_size (Variables|Decal|GetDecal%20Size))
  (bind _returnvalue (Transformation|GetWorldScale _defaultsceneroot))
  ;[1 1 1] 0)  Add single decal
  (if (Variables|Default|GetAdd%20Simple%20Decal)
    (bind _returnvalue_2 (AddComponent|AddDecalComponent false (Math|Transform|MakeTransform (Variables|Decal|GetSingle%20Decal%20Offset) (Math|Rotator|MakeRotator 0.0 -9e+01 (Variables|Decal|GetDecal%20Rotation)) (Math|Vector|MakeVector (* (.z _returnvalue) _decal_size) (* _decal_size (.y _returnvalue)) (* (.x _returnvalue) _decal_size)))))
    (Rendering|Components|Decal|SetDecalMaterial _returnvalue_2 (Variables|Decal|GetDecal%20Material))))

(fn AddMultiDecal
  (bind _single_decal_offset (Variables|Decal|GetSingle%20Decal%20Offset))
  (if (Variables|Default|GetAdd%20Multi-Decal)
    ;[1 1 1] 1) Add Multi decal
    (bind _output_get (Variables|Debug|SetDecal%20Amount+1 (Math|Float|Truncate (/ (Spline|GetSplineLength (Variables|Default|GetSpline)) (Variables|Decal|GetMulti%20Decal%20Section%20Size))))) ; DEBUG/Info Purposes
    (for _index (range 0 _output_get)
      (if (Variables|Debug|GetDebug%20Decal%20Position)
        (AddComponent|AddArrowComponent false (Math|Transform|MakeTransform (Spline|GetLocationatDistanceAlongSpline (Variables|Default|GetSpline) (* _index (Variables|Decal|GetMulti%20Decal%20Section%20Size)) "Local") (Math|Rotator|MakeRotator (.roll (Spline|GetRotationatDistanceAlongSpline (Variables|Default|GetSpline) (* _index (Variables|Decal|GetMulti%20Decal%20Section%20Size)) "Local")) (.pitch (Spline|GetRotationatDistanceAlongSpline (Variables|Default|GetSpline) (* _index (Variables|Decal|GetMulti%20Decal%20Section%20Size)) "Local")) (+ (.yaw (Spline|GetRotationatDistanceAlongSpline (Variables|Default|GetSpline) (* _index (Variables|Decal|GetMulti%20Decal%20Section%20Size)) "Local")) 0.0)) "1.000000,1.000000,1.000000")) ; debug
      )
      (bind _returnvalue (AddComponent|AddDecalComponent false (Math|Transform|MakeTransform (Spline|GetLocationatDistanceAlongSpline (Variables|Default|GetSpline) (* _index (Variables|Decal|GetMulti%20Decal%20Section%20Size)) "Local") (Math|Rotator|MakeRotator 0.0 -9e+01 (+ (.yaw (Spline|GetRotationatDistanceAlongSpline (Variables|Default|GetSpline) (* _index (Variables|Decal|GetMulti%20Decal%20Section%20Size)) "Local")) 0.0)) (CallFunction|GetDecalScale))))
      (bind _output_get_2 (Variables|Default|SetCurrent%20Decal _returnvalue))
      (Transformation|AddLocalRotation _output_get_2 (Math|Rotator|MakeRotator 0.0 0.0 (Variables|Decal|GetDecal%20Slope%20Factor)) false false)
      (if (Variables|Decal|GetShow%20MultiDecal%20Number)
        (bind _returnvalue_2 (AddComponent|AddTextRenderComponent false (Math|Transform|MakeTransform (Math|Vector|MakeVector (.x (* (Spline|GetLocationatDistanceAlongSpline (Variables|Default|GetSpline) (* _index (Variables|Decal|GetMulti%20Decal%20Section%20Size)) "Local") 1.0)) (.y (* (Spline|GetLocationatDistanceAlongSpline (Variables|Default|GetSpline) (* _index (Variables|Decal|GetMulti%20Decal%20Section%20Size)) "Local") 1.0)) (+ (.z (* (Spline|GetLocationatDistanceAlongSpline (Variables|Default|GetSpline) (* _index (Variables|Decal|GetMulti%20Decal%20Section%20Size)) "Local") 1.0)) 5e+03)) (Math|Rotator|MakeRotator (.roll (Spline|GetRotationatDistanceAlongSpline (Variables|Default|GetSpline) (* _index (Variables|Decal|GetMulti%20Decal%20Section%20Size)) "Local")) (.pitch (Spline|GetRotationatDistanceAlongSpline (Variables|Default|GetSpline) (* _index (Variables|Decal|GetMulti%20Decal%20Section%20Size)) "Local")) (+ (.yaw (Spline|GetRotationatDistanceAlongSpline (Variables|Default|GetSpline) (* _index (Variables|Decal|GetMulti%20Decal%20Section%20Size)) "Local")) 0.0)) "1.000000,1.000000,1.000000")))
        (Rendering|Components|TextRender|SetText _returnvalue_2 (Utilities|Text|ToText(Integer) _index)))
      (Transformation|AddLocalRotation (Variables|Default|GetCurrent%20Decal) (Math|Rotator|MakeRotator (Utilities|Select :Index _index :Option%200 (Variables|Decal|GetDecal%200%20Pitch) :Option%201 (Variables|Decal|GetDecal%201%20Pitch) :Option%202 (Variables|Decal|GetDecal%202%20Pitch) :Option%203 (Variables|Decal|GetDecal%203%20Pitch) :Option%204 (Variables|Decal|GetDecal%204%20Pitch) :Option%205 (Variables|Decal|GetDecal%205%20Pitch) :Option%206 (Variables|Decal|GetDecal%206%20Pitch) :Option%207 (Variables|Decal|GetDecal%207%20Pitch) :Option%208 (Variables|Decal|GetDecal%208%20Pitch) :Option%209 (Variables|Decal|GetDecal%209%20Pitch) :Option%2010 (Variables|Decal|GetDecal%2010%20Pitch) :Option%2011 (Variables|Decal|GetDecal%2011%20Pitch) :Option%2012 (Variables|Decal|GetDecal%2012%20Pitch) :Option%2013 (Variables|Decal|GetDecal%2013%20Pitch) :Option%2014 (Variables|Decal|GetDecal%2014%20Pitch) :Option%2015 (Variables|Decal|GetDecal%2015%20Pitch) :Option%2016 (Variables|Decal|GetDecal%2016%20Pitch) :Option%2017 (Variables|Decal|GetDecal%2017%20Pitch) :Option%2018 (Variables|Decal|GetDecal%2018%20Pitch) :Option%2019 (Variables|Decal|GetDecal%2019%20Pitch) :Option%2020 (Variables|Decal|GetDecal%2020%20Pitch) :Option%2021 (Variables|Decal|GetDecal%2021%20Pitch) :Option%2022 (Variables|Decal|GetDecal%2022%20Pitch) :Option%2023 (Variables|Decal|GetDecal%2023%20Pitch) :Option%2024 (Variables|Decal|GetDecal%2024%20Pitch) :Option%2025 (Variables|Decal|GetDecal%2025%20Pitch)) 0.0 0.0) false false)
      (Transformation|AddLocalOffset (Variables|Default|GetCurrent%20Decal) (Math|Vector|MakeVector (.z _single_decal_offset) (+ (Variables|Decal|GetDecal%20Pushout%20Factor) (.y _single_decal_offset)) (.x _single_decal_offset)) false false)
      (Rendering|Components|Decal|SetDecalMaterial (Variables|Default|GetCurrent%20Decal) (Variables|Decal|GetDecal%20Material)))))

(fn GetSplineStaticMesh
  (bind _randomstream (Variables|Default|GetRandomStream))
  (bind _meshtype (Variables|Default|GetMeshType))
  (bind _sequence_meshes (Variables|Default|GetSequence%20Meshes))
  (bind _mesh_sequence_number (Variables|Default|GetMesh%20Sequence%20Number))
  (bind _randomise_meshes (Variables|Default|GetRandomise%20Meshes))
  (bind _returnvalue (Math|Random|RandomIntegerinRangefromStream 0 1 _randomstream))
  (bind _returnvalue_2 (Math|Random|RandomIntegerinRangefromStream 0 2 _randomstream))
  (bind _returnvalue_3 (select _sequence_meshes _mesh_sequence_number 0))
  (bind _returnvalue_4 (Utilities|Select :Index _meshtype :NewEnumerator0 _returnvalue_2 :NewEnumerator1 0 :NewEnumerator2 0 :NewEnumerator5 _returnvalue_2 :NewEnumerator3 0 :NewEnumerator4 _returnvalue_2 :NewEnumerator7 0 :NewEnumerator6 _returnvalue :NewEnumerator8 0))
  (bind _returnvalue_5 (select _randomise_meshes _returnvalue_4 _returnvalue_3))
  ;[1 1 1] Select Mesh
  (return (Utilities|Select :Index (Variables|Default|GetMeshType) :NewEnumerator0 (Utilities|Select :Index _returnvalue_5 :Option%200 "/Game/RealBiomes/Meshes/Cliffs/Desert_Cliff_Large/SM_Desert_Cliff_Large_Wall_01.SM_Desert_Cliff_Large_Wall_01" :Option%201 "/Game/RealBiomes/Meshes/Cliffs/Desert_Cliff_Large/SM_Desert_Cliff_Large_Wall_02.SM_Desert_Cliff_Large_Wall_02" :Option%202 "/Game/RealBiomes/Meshes/Cliffs/Desert_Cliff_Large/SM_Desert_Cliff_Large_Wall_03.SM_Desert_Cliff_Large_Wall_03") :NewEnumerator1 "/Game/RealBiomes/Meshes/Cliffs/Desert_Cliff_Small/SM_Desert_Cliff_Small_01.SM_Desert_Cliff_Small_01" :NewEnumerator2 "/Game/RealBiomes/Meshes/Cliffs/Desert_Cliff_Small/SM_Desert_Cliff_Small_02_A.SM_Desert_Cliff_Small_02_A" :NewEnumerator5 (Utilities|Select :Index _returnvalue_5 :Option%200 "/Game/RealBiomes/Meshes/Cliffs/Desert_Cliff_Small/SM_Desert_Cliff_Small_02_B.SM_Desert_Cliff_Small_02_B" :Option%201 "/Game/RealBiomes/Meshes/Cliffs/Desert_Cliff_Small/SM_Desert_Cliff_Small_02_C.SM_Desert_Cliff_Small_02_C" :Option%202 "/Game/RealBiomes/Meshes/Cliffs/Desert_Cliff_Small/SM_Desert_Cliff_Small_02_D.SM_Desert_Cliff_Small_02_D") :NewEnumerator3 "/Game/RealBiomes/Meshes/Cliffs/Desert_Cliff_Small/SM_Desert_Cliff_Small_03_A.SM_Desert_Cliff_Small_03_A" :NewEnumerator4 (Utilities|Select :Index _returnvalue_5 :Option%200 "/Game/RealBiomes/Meshes/Cliffs/Desert_Cliff_Small/SM_Desert_Cliff_Small_03_B.SM_Desert_Cliff_Small_03_B" :Option%201 "/Game/RealBiomes/Meshes/Cliffs/Desert_Cliff_Small/SM_Desert_Cliff_Small_03_C.SM_Desert_Cliff_Small_03_C" :Option%202 "/Game/RealBiomes/Meshes/Cliffs/Desert_Cliff_Small/SM_Desert_Cliff_Small_03_D.SM_Desert_Cliff_Small_03_D") :NewEnumerator7 "/Game/RealBiomes/Meshes/Cliffs/Desert_Cliff_Small/SM_Desert_Cliff_Small_04_A.SM_Desert_Cliff_Small_04_A" :NewEnumerator6 (Utilities|Select :Index (Math|Integer|Clamp(Integer) _returnvalue_5 0 1) :Option%200 "/Game/RealBiomes/Meshes/Cliffs/Desert_Cliff_Small/SM_Desert_Cliff_Small_04_B.SM_Desert_Cliff_Small_04_B" :Option%201 "/Game/RealBiomes/Meshes/Cliffs/Desert_Cliff_Small/SM_Desert_Cliff_Small_04_C.SM_Desert_Cliff_Small_04_C") :NewEnumerator8 (Variables|Default|GetCustom%20Mesh))))

(fn GetSplineMeshPositionandTangents
  (bind _spline (Variables|Default|GetSpline))
  (bind _is_closed_loop (Variables|Default|GetIs%20Closed%20Loop))
  (bind _spline_2 (Variables|Default|GetSpline))
  (bind _is_closed_loop_2 (Variables|Default|GetIs%20Closed%20Loop))
  (bind _shift (Variables|Default|Getshift))
  (bind _is_closed_loop_3 (Variables|Default|GetIs%20Closed%20Loop))
  (bind _offset_start_position (Variables|Advanced:GapOffsets|GetOffset%20Start%20Position))
  (bind _offset_end_pos (Variables|Advanced:GapOffsets|GetOffset%20End%20Pos))
  (bind _flip_mesh (Variables|Default|GetFlip%20Mesh))
  (bind _flip_mesh_2 (Variables|Default|GetFlip%20Mesh))
  (bind _splinelength (Variables|Default|GetSplineLength))
  (bind _splinelength_2 (Variables|Default|GetSplineLength))
  (bind _is_closed_loop_4 (Variables|Default|GetIs%20Closed%20Loop))
  (bind _splinelength_3 (Variables|Default|GetSplineLength))
  (bind _splinelength_4 (Variables|Default|GetSplineLength))
  (bind _sectionlength_current (Variables|Default|GetSectionLength_Current))
  (bind _splinelength_5 (Variables|Default|GetSplineLength))
  (bind _corrected_section_length (Variables|Default|GetCorrected%20Section%20Length))
  (bind _splinelength_6 (Variables|Default|GetSplineLength))
  (bind _shift_2 (Variables|Default|Getshift))
  (bind _sectionlength_current_2 (Variables|Default|GetSectionLength_Current))
  (bind _returnvalue (- _sectionlength_current _offset_start_position))
  (bind _returnvalue_2 (select _is_closed_loop_3 _shift 0.0))
  (bind _returnvalue_3 (select _is_closed_loop _shift_2 0.0))
  (bind _returnvalue_4 (+ _returnvalue _returnvalue_3))
  (bind _returnvalue_5 (+ _offset_end_pos _sectionlength_current_2 _corrected_section_length _returnvalue_2))
  (bind _returnvalue_6 (Math|Float|%(Float) _returnvalue_5 _splinelength_3))
  (bind _returnvalue_7 (> _returnvalue_4 _splinelength_4))
  (bind _returnvalue_8 (Math|Float|%(Float) _returnvalue_4 _splinelength_5))
  (bind _returnvalue_9 (> _returnvalue_5 _splinelength_6))
  (bind _returnvalue_10 (and _returnvalue_7 _is_closed_loop_4))
  (bind _returnvalue_11 (and _returnvalue_9 _is_closed_loop_2))
  (bind _returnvalue_12 (select _returnvalue_11 _returnvalue_6 _returnvalue_5))
  (bind _returnvalue_13 (select _returnvalue_10 _returnvalue_8 _returnvalue_4))
  (bind _returnvalue_14 (Math|Float|Clamp(Float) _returnvalue_12 0.0 _splinelength))
  (bind _returnvalue_15 (Math|Float|Clamp(Float) _returnvalue_13 0.0 _splinelength_2))
  (bind _returnvalue_16 (select _flip_mesh_2 _returnvalue_15 _returnvalue_14))
  (bind _returnvalue_17 (select _flip_mesh _returnvalue_14 _returnvalue_15))
  (bind _returnvalue_18 (Spline|GetTangentatDistanceAlongSpline _spline _returnvalue_16 "Local"))
  (bind _returnvalue_19 (Spline|GetTangentatDistanceAlongSpline _spline_2 _returnvalue_17 "Local"))
  (return (Spline|GetLocationatDistanceAlongSpline (Variables|Default|GetSpline) _returnvalue_17 "Local") (Spline|GetLocationatDistanceAlongSpline (Variables|Default|GetSpline) _returnvalue_16 "Local") (Math|Vector|ClampVectorSize (select (Variables|Default|GetBend%20Meshes) (select (Variables|Default|GetFlip%20Mesh) (* _returnvalue_19 -1.0) _returnvalue_19) "0, 0, 0") 0.0 (Variables|Default|GetCorrected%20Section%20Length)) (Math|Vector|ClampVectorSize (select (Variables|Default|GetBend%20Meshes) (select (Variables|Default|GetFlip%20Mesh) (* _returnvalue_18 -1.0) _returnvalue_18) "0, 0, 0") 0.0 (Variables|Default|GetCorrected%20Section%20Length))))

(fn CacheSplinePointLocation)