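; BP_Drone_Create is a placement actor that fills a 3D grid with BP_Drone child actors.
; Its Construction Script loops over NumberX, NumberY and NumberZ, adding one child actor component per cell while the event graph stays empty.
; Each cell index is multiplied by a random spacing bounded by Distance and RandomLocation, then shifted by forward and right vector offsets for centering.
; Every drone also gets random yaw and scale.
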(event EventBeginPlay)

(event Collision|EventActorBeginOverlap
  (params (OtherActor :type Actor%20Object%20Reference)))

(event EventTick
  (params (DeltaSeconds :type Float%20%28single-precision%29)))

(fn ConstructionScript
  (bind _returnvalue (Math|Random|RandomFloatinRange 1.2 1.5))
  (bind _randomlocation (Variables|Default|GetRandomLocation))
  (bind _distance (Variables|Default|GetDistance))
  (bind _numberzarray (Variables|Default|GetNumberZArray))
  (bind _numbery (Variables|Default|GetNumberY))
  (bind _returnvalue_2 (* _distance _randomlocation))
  (bind _returnvalue_3 (Math|Random|RandomFloatinRange _returnvalue_2 _distance))
  (Utilities|Array|Resize _numberzarray (Variables|Default|GetNumberZ))
  (for (_ _array_index) _numberzarray
    (for _index (range 0 (- (* (Variables|Default|GetNumberX) (Variables|Default|GetNumberY)) 1))
      (bind _returnvalue_4 (AddComponent|AddChildActorComponent false (Math|Transform|MakeTransform (- (Math|Vector|MakeVector (* (/ _index _numbery) _returnvalue_3) (* _returnvalue_3 (Math|Integer|%(Integer) _index _numbery)) (* _returnvalue_3 _array_index)) (+ (/ (* (- (Variables|Default|GetNumberY) 1) (* (Transformation|GetActorForwardVector) _distance)) 2.0) (/ (* (- (Variables|Default|GetNumberX) 1) (* (Transformation|GetActorRightVector) _distance)) 2.0))) (Math|Rotator|MakeRotator 0.0 0.0 (Math|Random|RandomFloatinRange 0.0 3.6e+02)) (Math|Vector|MakeVector _returnvalue _returnvalue _returnvalue))))
      (ChildActorComponent|SetChildActorClass _returnvalue_4 "/Game/Blueprint/Monster/BP_Drone.BP_Drone_C"))))