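; Actor component that drives a character's flight: sprint and aim modes switch fly speed, acceleration, rotation rate and orient-to-movement.
; Tick derives movement input, sprint vertical speed and smoothed lean from velocity rotation deltas, exposed through getters.
; Hits while sprinting cancel sprint; ground hits at certain camera pitches stop flight and level the view (superhero landing), gated by DoOnce until StartFlight.
; Camera rotation and spring arm offset/length ease via Delay(0) loops.
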(event Custom|SetSprintEvent
  (params (IsSprint :type Boolean))
  (State|SetIsSprintFunc IsSprint))

(event Custom|SetAimingEvent
  (params (IsAiming :type Boolean))
  (State|SetIsAimingFunc IsAiming))

(event Custom|HitEvent
  (params (SelfActor :type Actor%20Object%20Reference) (OtherActor :type Actor%20Object%20Reference) (NormalImpulse :type Vector) (Hit :type Hit%20Result%20Structure%20%28by%20ref%29))
  ;[1 1 1] Hit Event Binding and Superhero landing logic.
  (Utilities|FlowControl|Sequence
    (:then_0
      (|HitEventCollapseGraph Hit))
    (:then_1
      (Variables|State|SetIsHit true)
      (Utilities|FlowControl|Delay 1.0)
      (Variables|State|SetIsHit false))))

(event EventTick
  (params (DeltaSeconds :type Float%20%28single-precision%29))
  ;[1 1 1] Tick Event
  (|FlightUpdateCollapseGraph))

(event EventBeginPlay
  ;[1 1 1] Begin Play
  (|BeginPlayCollapseGraph)
  ;[1 1 1] Hit Event Binding and Superhero landing logic.
  (Collision|AssignOnActorHit (Variables|References|GetCharacter) (delegate Custom|HitEvent)))

(fn SetIsSprintFunc
  (params (IsSprint :type Boolean))
  (bind _charactermovement (Variables|References|GetCharacterMovement))
  (bind _charactermovement_2 (Variables|References|GetCharacterMovement))
  (bind _charactermovement_3 (Variables|References|GetCharacterMovement))
  (if true
    (bind _output_get (Variables|State|SetIsSprint IsSprint))
    (Variables|/Script/Engine.CharacterMovementComponent|SetbOrientRotationToMovement (Variables|References|GetCharacterMovement) (not _output_get))
    (if IsSprint
      (Variables|/Script/Engine.CharacterMovementComponent|SetMaxFlySpeed _charactermovement_3 (Variables|ParametersSetting|GetSprintFlySpeed))
      (Variables|/Script/Engine.CharacterMovementComponent|SetMaxAcceleration _charactermovement (Variables|ParametersSetting|GetSprintAcceleration))
      (Variables|/Script/Engine.CharacterMovementComponent|SetRotationRate _charactermovement_2 (Variables|ParametersSetting|GetSprintRotationRate))
      (CallFunction|StartFlight)
      (else
        (Variables|/Script/Engine.CharacterMovementComponent|SetMaxFlySpeed _charactermovement_3 (Variables|ParametersSetting|GetHoverFlySpeed))
        (Variables|/Script/Engine.CharacterMovementComponent|SetMaxAcceleration _charactermovement (Variables|ParametersSetting|GetHoverAcceleration))
        (Variables|/Script/Engine.CharacterMovementComponent|SetRotationRate _charactermovement_2 (Variables|ParametersSetting|GetHoverRotationRate))))))

(fn GetIsSprintFunc
  (return (Variables|State|GetIsSprint)))

(fn SetFlightMovementParamFunc
  (Variables|/Script/Engine.CharacterMovementComponent|SetMaxFlySpeed (Variables|References|GetCharacterMovement) (Variables|ParametersSetting|GetHoverFlySpeed))
  (Variables|/Script/Engine.CharacterMovementComponent|SetMaxAcceleration (Variables|References|GetCharacterMovement) (Variables|ParametersSetting|GetHoverAcceleration))
  (Variables|/Script/Engine.CharacterMovementComponent|SetRotationRate (Variables|References|GetCharacterMovement) (Variables|ParametersSetting|GetHoverRotationRate)))

(fn SetIsAimingFunc
  (params (IsAiming :type Boolean))
  (bind _springarm (Variables|References|GetSpringArm))
  (bind _springarm_2 (Variables|References|GetSpringArm))
  (if IsAiming
    ;[1 1 1] Aiming settings True
    (Variables|State|SetIsAiming true)
    (Variables|/Script/Engine.CharacterMovementComponent|SetbOrientRotationToMovement (Variables|References|GetCharacterMovement) false)
    (Variables|/Script/Engine.CharacterMovementComponent|SetMaxFlySpeed (Variables|References|GetCharacterMovement) (* (Variables|ParametersSetting|GetHoverFlySpeed) 0.3))
    (Variables|/Script/Engine.SpringArmComponent|SetbEnableCameraLag _springarm_2 true)
    (Variables|/Script/Engine.SpringArmComponent|SetbEnableCameraRotationLag _springarm_2 true)
    (else
      ;[1 1 1] Aiming settings False
      (Variables|State|SetIsAiming false)
      (Variables|/Script/Engine.CharacterMovementComponent|SetbOrientRotationToMovement (Variables|References|GetCharacterMovement) true)
      (Variables|/Script/Engine.CharacterMovementComponent|SetMaxFlySpeed (Variables|References|GetCharacterMovement) (Variables|ParametersSetting|GetHoverFlySpeed))
      (Variables|/Script/Engine.SpringArmComponent|SetbEnableCameraLag _springarm true)
      (Variables|/Script/Engine.SpringArmComponent|SetbEnableCameraRotationLag _springarm true))))

(fn GetHighSpeedVerticalSpeedFunc
  (return (Variables|Move|GetHighSpeedVerticalSpeed)))

(fn GetLeanParameterFunc
  (return (Variables|Move|GetLean)))

(fn GetIsAimingFunc
  (return (Variables|State|GetIsAiming)))

(fn SetHasMovementInputFunc
  (params (HasMovementInput :type Boolean))
  (Variables|State|SetHasMovementInput HasMovementInput))

(fn GetHasMovementInputFunc
  (return (Variables|State|GetHasMovementInput)))

(event Custom|ResetLandingEventDoOnce
  (bind _character (Variables|References|GetCharacter))
  (bind _character_2 (Variables|References|GetCharacter))
  (bind _returnvalue (Pawn|GetControlRotation _character_2 :!class /Script/Engine.Pawn))
  (bind _returnvalue_2 (Pawn|GetControlRotation _character :!class /Script/Engine.Pawn))
  ;[1 1 1] When the camera hits the ground while sprinting at a certain angle, it makes a superhero landing.
  (Utilities|FlowControl|Sequence
    (:then_0
      (Utilities|FlowControl|DoOnce false) ; enters at Reset
    )
    (:then_1
      (Utilities|FlowControl|DoOnce false) ; enters at Reset
    )))

(event Custom|StartFlight
  ;[1 1 1] Event to start the flight and stop the flight.
  (CallFunction|ResetLandingEventDoOnce))

(event Custom|StopFlight
  ;[1 1 1] Event to start the flight and stop the flight.
  (State|SetIsSprintFunc false))

(event Custom|Set%20Spring%20Arm
  (params (Target%20%20Length :type Float%20%28double-precision%29) (Target%20Socket%20Offset :type Vector :default "0.000000,0.000000,50.000000") (Socket%20Offset%20Speed :type Float%20%28double-precision%29))
  (Variables|Camera|SetTargetSocketOffset Target%20Socket%20Offset)
  (Variables|Camera|SetTargetLength Target%20%20Length)
  (Variables|Camera|SetInterpSpeed Socket%20Offset%20Speed)
  (Utilities|FlowControl|Sequence
    (:then_0
      ;[0 0 0] 弹簧臂位移
      (if (not (Utilities|Operators|EqualEqual (Variables|/Script/Engine.SpringArmComponent|GetSocketOffset (Variables|References|GetSpringArm)) (Variables|Camera|GetTargetSocketOffset) 1.0)) :!label _label
        (Utilities|FlowControl|Sequence
          (:then_0
            (Variables|/Script/Engine.SpringArmComponent|SetSocketOffset (Variables|References|GetSpringArm) (Math|Interpolation|VInterpTo (Variables|/Script/Engine.SpringArmComponent|GetSocketOffset (Variables|References|GetSpringArm)) (Variables|Camera|GetTargetSocketOffset) (Utilities|Time|GetWorldDeltaSeconds) (Variables|Camera|GetInterpSpeed))))
          (:then_1
            (Utilities|FlowControl|Delay 0.0)
            (goto _label)))))
    (:then_1
      ;[0 0 0] 弹簧臂长度
      (if (not (Math|Float|NearlyEqual(Float) (Variables|/Script/Engine.SpringArmComponent|GetTargetArmLength (Variables|References|GetSpringArm)) (Variables|Camera|GetTargetLength) 1.0)) :!label _label_2
        (Utilities|FlowControl|Sequence
          (:then_0
            (Variables|/Script/Engine.SpringArmComponent|SetTargetArmLength (Variables|References|GetSpringArm) (Math|Interpolation|FInterpTo (Variables|/Script/Engine.SpringArmComponent|GetTargetArmLength (Variables|References|GetSpringArm)) (Variables|Camera|GetTargetLength) (Utilities|Time|GetWorldDeltaSeconds) (Variables|Camera|GetInterpSpeed))))
          (:then_1
            (Utilities|FlowControl|Delay 0.0)
            (goto _label_2)))))))

(event Custom|SetCamera
  (params (CameraRotator :type Rotator) (CameraRotatorSpeed :type Float%20%28single-precision%29))
  ;[0 0 0] 相机旋转
  (Variables|Camera|SetTargetCameraRotator CameraRotator)
  (Variables|Camera|SetCameraRotatorSpeed CameraRotatorSpeed)
  (if (not (Utilities|Operators|EqualEqual (Variables|/Script/Engine.SceneComponent|GetRelativeRotation (Variables|References|GetCamera)) (Variables|Camera|GetTargetCameraRotator) 0.5)) :!label _label
    (Utilities|FlowControl|Sequence
      (:then_0
        (Transformation|SetRelativeRotation (Variables|References|GetCamera) (Math|Interpolation|RInterpTo (Variables|/Script/Engine.SceneComponent|GetRelativeRotation (Variables|References|GetCamera)) (Variables|Camera|GetTargetCameraRotator) (Utilities|Time|GetWorldDeltaSeconds) (Variables|Camera|GetCameraRotatorSpeed)) false false))
      (:then_1
        (Utilities|FlowControl|Delay 0.0)
        (goto _label)))))