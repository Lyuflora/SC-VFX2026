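; Player character Blueprint for Nyx, a flying role with hover movement, sprint, aiming and a five-step melee combo.
; Input delegates sprint, aim and spring-arm changes to BPCMotionComponent, while movement follows control rotation plus a vertical axis.
; When idle, a camera-driven head look-at limits mouse yaw around the actor's facing.
; Left-click queues combo montages, with a timeline resetting the chain; T debug-spawns a Bezier bullet.
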(event EventBeginPlay
  (bind _returnvalue (Game|GetPlayerCameraManager 0))
  ;[0 0 0] 设置相机上下朝向
  (Variables|/Script/Engine.PlayerCameraManager|SetViewPitchMin _returnvalue -7e+01)
  (Variables|/Script/Engine.PlayerCameraManager|SetViewPitchMax _returnvalue 7e+01)
  (Transformation|SetActorRotation (Transformation|GetWorldRotation (Variables|Character|GetMesh))))

(event EventTick
  (params (DeltaSeconds :type Float%20%28single-precision%29))
  (bind _returnvalue (Transformation|GetActorRotation))
  (bind _camera (Variables|Default|GetCamera))
  ;[0 0 0] 头部LookAt位置
  (Utilities|FlowControl|Sequence
    (:then_0
      (Variables|Input|SetLookAtLocation (+ (Transformation|GetWorldLocation _camera) (* (Math|Rotator|GetRotationXVector (Transformation|GetWorldRotation _camera)) 1e+04))))
    (:then_1
      ;[0 0 0] 设置LookAt左右旋转值
      (if (Math|Boolean|ANDBoolean (== (Variables|Input|GetMoveForwardValue) 0.0) (== (Variables|Input|GetMoveRightValue) 0.0) (not (Default|GetIsSprintFunc (Variables|Default|GetBPC_MotionComponent))))
        (Variables|Input|SetIsLookAt true)
        (Variables|Input|SetMaxYaw (+ (.yaw _returnvalue) 8e+01))
        (Variables|Input|SetMinYaw (- (.yaw _returnvalue) 8e+01))
        (else
          (Variables|Input|SetIsLookAt false))))))

(event Input|ActionEvents|InputActionSprint
  (params (Key :type Key%20Structure :default "None"))
  (bind _bpc_motioncomponent (Variables|Default|GetBPC_MotionComponent))
  ;[0 0 0] Sprint
  (:Pressed
    (if (not (Math|Boolean|ORBoolean (Variables|Attack|GetIsSkill) (Variables|Attack|GetIsAttacking) (Default|GetIsAimingFunc (Variables|Default|GetBPC_MotionComponent))))
      (Default|SetSprintEvent _bpc_motioncomponent true)))
  (:Released
    (Default|SetSprintEvent _bpc_motioncomponent false)))

(event Input|ActionEvents|InputActionAim
  (params (Key :type Key%20Structure :default "None"))
  (bind _animmontage (Variables|Default|GetAnimMontage))
  (bind _bpc_motioncomponent (Variables|Default|GetBPC_MotionComponent))
  (bind _aimstart (Utilities|Struct|BreakST_AnimMontage _animmontage))
  ;[1 1 1] Aiming
  (:Pressed
    (if (not (Default|GetIsSprintFunc (Variables|Default|GetBPC_MotionComponent)))
      (Variables|Input|SetIsAim true)
      (Animation|PlayAnimMontage _aimstart 1.0 "None")
      (Default|SetAimingEvent _bpc_motioncomponent true)
      (Default|SetSpringArm _bpc_motioncomponent 2e+02 "0.000000,100.000000,20.000000" 5.0)))
  (:Released
    (Variables|Input|SetIsAim false)
    (Animation|StopAnimMontage _aimstart)
    (Default|SetAimingEvent _bpc_motioncomponent false)
    (Default|SetSpringArm _bpc_motioncomponent 3e+02 "0.000000,0.000000,50.000000" 5.0)))

(event Input|ActionEvents|InputActionDodge
  (params (Key :type Key%20Structure :default "None"))
  ;[1 1 1] Dodge
)

(event Input|AxisEvents|InputAxisMoveUp/Down
  (params (AxisValue :type Float%20%28single-precision%29))
  ;[0 0 0] MoveUp/Down
  (if (and (Variables|Input|GetCanMove) (not (Default|GetIsSprintFunc (Variables|Default|GetBPC_MotionComponent))))
    (Pawn|Input|AddMovementInput (Math|Vector|GetUpVector (Transformation|GetActorRotation)) AxisValue false)))

(event Input|AxisEvents|InputAxisMoveForward/Backward
  (params (AxisValue :type Float%20%28single-precision%29))
  (bind _returnvalue (Pawn|GetControlRotation :!class /Script/Engine.Pawn))
  (bind _returnvalue_2 (Math|Rotator|GetRotationXVector _returnvalue))
  ;[0 0 0] Movement
  (bind _output_get (Variables|Input|SetMoveForwardValue AxisValue))
  (if (Variables|Input|GetCanMove)
    (Pawn|Input|AddMovementInput (Math|Vector|MakeVector (.x _returnvalue_2) (.y _returnvalue_2) (+ (select (Math|Float|InRange(Float) (.z _returnvalue_2) -1.0 -0.1) (.z _returnvalue_2) 0.0) (select (Math|Float|InRange(Float) (.z _returnvalue_2) 0.1 1.0) (.z _returnvalue_2) 0.0))) (select (Default|GetIsSprintFunc (Variables|Default|GetBPC_MotionComponent)) 1.0 _output_get) false)))

(event Input|AxisEvents|InputAxisTurnRight/LeftMouse
  (params (AxisValue :type Float%20%28single-precision%29))
  (bind _returnvalue (Pawn|GetControlRotation :!class /Script/Engine.Pawn))
  ;[0 0 0] Camera Input - Mouse
  (if (Variables|Input|GetIsLookAt)
    (if (> (Math|Vector|DotProduct (Math|Rotator|GetRotationXVector (Pawn|GetControlRotation :!class /Script/Engine.Pawn)) (Math|Rotator|GetRotationXVector (Transformation|GetActorRotation))) 0.0)
      (Pawn|SetControlRotation (Game|GetPlayerController 0) (Math|Rotator|MakeRotator (.roll _returnvalue) (.pitch _returnvalue) (Class|KismetMathLibrary|ClampAxis (Math|Float|ClampAngle (+ (.yaw _returnvalue) AxisValue) (Variables|Input|GetMinYaw) (Variables|Input|GetMaxYaw)))))
      (else
        (Pawn|Input|AddControllerYawInput AxisValue :!label _label)))
    (else
      (goto _label))))

(event Input|AxisEvents|InputAxisLookUp/DownMouse
  (params (AxisValue :type Float%20%28single-precision%29))
  ;[0 0 0] Camera Input - Mouse
  (Pawn|Input|AddControllerPitchInput AxisValue))

(event Input|AxisEvents|InputAxisMoveRight/Left
  (params (AxisValue :type Float%20%28single-precision%29))
  (bind _bpc_motioncomponent (Variables|Default|GetBPC_MotionComponent))
  (bind _issprint (Default|GetIsSprintFunc _bpc_motioncomponent))
  ;[0 0 0] Movement
  (bind _output_get (Variables|Input|SetMoveRightValue AxisValue))
  (if (Variables|Input|GetCanMove)
    (if (not _issprint)
      (Pawn|Input|AddMovementInput (select _issprint "0, 0, 0" (Math|Vector|GetRightVector (Math|Rotator|MakeRotator 0.0 0.0 (.Yaw (Math|Rotator|BreakRotator (Pawn|GetControlRotation :!class /Script/Engine.Pawn)))))) _output_get false))))

(event Input|KeyboardEvents|Q
  (params (Key :type Key%20Structure :default "None"))
  (bind _charactermovement (Variables|Character|GetCharacterMovement))
  ;[0 0 0] MoveUp/Down
  (:Pressed
    (Variables|/Script/Engine.CharacterMovementComponent|SetbOrientRotationToMovement _charactermovement false :!label _label))
  (:Released
    (if (Default|GetIsAimingFunc (Variables|Default|GetBPC_MotionComponent))
      (goto _label)
      (else
        (Variables|/Script/Engine.CharacterMovementComponent|SetbOrientRotationToMovement _charactermovement true)))))

(event Input|KeyboardEvents|E
  (params (Key :type Key%20Structure :default "None"))
  (bind _charactermovement (Variables|Character|GetCharacterMovement))
  ;[0 0 0] MoveUp/Down
  (:Pressed
    (Variables|/Script/Engine.CharacterMovementComponent|SetbOrientRotationToMovement _charactermovement false :!label _label))
  (:Released
    (if (Default|GetIsAimingFunc (Variables|Default|GetBPC_MotionComponent))
      (goto _label)
      (else
        (Variables|/Script/Engine.CharacterMovementComponent|SetbOrientRotationToMovement _charactermovement true)))))

(event Input|KeyboardEvents|T
  (params (Key :type Key%20Structure :default "None"))
  ;[1 1 1] Spawn Bullet
  (:Pressed
    (Game|SpawnActorfromClass "/Game/Effect/Blueprint/EF_BP_Basic_BezierBullet.EF_BP_Basic_BezierBullet_C" (Transformation|GetActorTransform) "Undefined" 0 0)
    (Development|PrintString "Spawn Bullet")))

(event Custom|ComboAttack
  (bind _animmontage (Variables|Default|GetAnimMontage))
  (bind (_combo1 _combo2 _combo3 _combo4 _combo5) (Utilities|Struct|BreakST_AnimMontage _animmontage))
  ;[0 0 0] Combo
  (if (Variables|Attack|GetReadyToCombo)
    (Variables|Attack|SetReadyToCombo false)
    (switch int (Variables|Attack|GetComboNumber)
      (:0
        (Variables|Attack|SetComboNumber 1)
        (Variables|Attack|SetComboMontage _combo1))
      (:1
        (Variables|Attack|SetComboNumber 2)
        (Variables|Attack|SetComboMontage _combo2))
      (:2
        (Variables|Attack|SetComboNumber 3)
        (Variables|Attack|SetComboMontage _combo3)
        (Utilities|FlowControl|Sequence
          (:then_0
            _)))
      (:3
        (Variables|Attack|SetComboNumber 4)
        (Variables|Attack|SetComboMontage _combo4)
        (Utilities|FlowControl|Sequence
          (:then_0
            _)))
      (:4
        (Variables|Attack|SetComboNumber 5)
        (Variables|Attack|SetComboMontage _combo5)
        (Utilities|FlowControl|Sequence
          (:then_0
            (Variables|Attack|SetIsAttacking false)))))
    (Animation|PlayAnimMontage (Variables|Attack|GetComboMontage) 1.0 "None")))

(event Custom|Is%20Attack
  (bind _animmontage (Variables|Default|GetAnimMontage))
  (bind (_combo1 _combo2 _combo3 _combo4 _combo5) (Utilities|Struct|BreakST_AnimMontage _animmontage))
  ;[0 0 0] Combo
  (if (not (or (Default|GetIsSprintFunc (Variables|Default|GetBPC_MotionComponent)) (Variables|Attack|GetIsSkill)))
    (if (Variables|Attack|GetIsAttacking)
      (Variables|Attack|SetReadyToCombo true)
      (else
        (Variables|Attack|SetIsAttacking true)
        (Utilities|CheakAttackM 3e+02 false)
        (switch int (Variables|Attack|GetComboNumber)
          (:0
            (Variables|Attack|SetComboNumber 1)
            (Variables|Attack|SetComboMontage _combo1))
          (:1
            (Variables|Attack|SetComboNumber 2)
            (Variables|Attack|SetComboMontage _combo2))
          (:2
            (Variables|Attack|SetComboNumber 3)
            (Variables|Attack|SetComboMontage _combo3)
            (Utilities|FlowControl|Sequence
              (:then_0
                _)))
          (:3
            (Variables|Attack|SetComboNumber 4)
            (Variables|Attack|SetComboMontage _combo4)
            (Utilities|FlowControl|Sequence
              (:then_0
                _)))
          (:4
            (Variables|Attack|SetComboNumber 5)
            (Variables|Attack|SetComboMontage _combo5)
            (Utilities|FlowControl|Sequence
              (:then_0
                (Variables|Attack|SetIsAttacking false)))))
        (Animation|PlayAnimMontage (Variables|Attack|GetComboMontage) 1.0 "None")))))

(event Custom|ResetAttack
  (params (DelayReadyToCombo :type Float%20%28single-precision%29))
  ;[0 0 0] Combo
  (Components|Timeline|SetTimelineLength (Variables|Default|GetTimeline_ResetCombo) DelayReadyToCombo)
  (Variables|Attack|SetIsAttacking false)
  (Timeline|Timeline_ResetCombo PlayFromStart
    (:Finished
      (Variables|Attack|SetReadyToCombo false)
      (Variables|Attack|SetComboNumber 0)
      (Utilities|ResetAttackM))))

(event Input|MouseEvents|LeftMouseButton
  (params (Key :type Key%20Structure :default "None"))
  ;[0 0 0] Combo
  (:Pressed
    (Audio|Components|Audio|Stop (Variables|Default|GetTimeline_ResetCombo))
    (Variables|Attack|SetReadyToCombo false)
    (CallFunction|IsAttack)))

(fn ConstructionScript)