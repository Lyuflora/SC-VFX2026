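; Bullet actor that flies along a randomized cubic Bezier curve from its spawn point to a target 30 m along the camera's forward vector.
; On BeginPlay it rolls random angles for two control points, which are pushed sideways around the start-to-target axis.
; A timeline drives the lerp, evaluating the curve by recursive point interpolation (De Casteljau) and rotating the actor to face each new position.
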(event EventBeginPlay
  (bind _returnvalue (Transformation|GetActorLocation))
  (Variables|Default|SetLocationStart _returnvalue)
  (Variables|Default|SetLocationEnd (+ _returnvalue (* (Transformation|GetActorForwardVector (Game|GetPlayerCameraManager 0)) 3e+03)))
  (Variables|Default|SetPoint2Width 5e+02)
  (Variables|Default|SetLocation2Rotation (Math|Random|RandomFloatinRange 0.0 3.6e+02))
  (Variables|Default|SetLocation3Rotation (Math|Random|RandomFloatinRange 0.0 3.6e+02))
  (bind _lerp (Timeline|Timeline_BezierMove PlayFromStart)
    (:Update
      (CallFunction|BezierLocationGenerator (Variables|Default|GetLocationEnd) _lerp))))

(event Collision|EventActorBeginOverlap
  (params (OtherActor :type Actor%20Object%20Reference)))

(event EventTick
  (params (DeltaSeconds :type Float%20%28single-precision%29)))

(fn ConstructionScript
  (|CallParentFunction))

(fn BezierMove
  (params (LocationArray :type Array%20of%20Vectors) (Lerp :type Float%20%28double-precision%29))
  (bind _returnvalue (Utilities|Array|Length LocationArray))
  (if (<= _returnvalue 1)
    (return (Utilities|Array|Get(acopy) LocationArray))
    (else
      (for _index (range 0 (- _returnvalue 2))
        (Utilities|Array|Add (LocalVariables|GetLocalLocationArray) (Math|Vector|Lerp(Vector) (Utilities|Array|Get(acopy) LocationArray _index) (Utilities|Array|Get(acopy) LocationArray (+ _index 1)) Lerp)))
      (bind _result (CallFunction|BezierMove (LocalVariables|GetLocalLocationArray) Lerp))
      (return _result))))

(fn BezierLocationGenerator
  (params (TargetLocation :type Vector) (Lerp :type Float%20%28double-precision%29))
  (bind _locationstart (Variables|Default|GetLocationStart))
  (bind _returnvalue (CallFunction|ControlPointCalculator _locationstart TargetLocation 0.3 (Variables|Default|GetLocation2Rotation) (Variables|Default|GetPoint2Width))) ; Point 2
  (bind _returnvalue_2 (CallFunction|ControlPointCalculator _locationstart TargetLocation 0.65 (Variables|Default|GetLocation3Rotation) (Variables|Default|GetPoint3Width))) ; Point 3
  (bind _result (CallFunction|BezierMove (Utilities|Array|MakeArray _locationstart _returnvalue _returnvalue_2 TargetLocation) Lerp))
  (Transformation|SetActorLocationAndRotation _result (Math|Rotator|FindLookatRotation (Transformation|GetActorLocation) _result)))

(fn ControlPointCalculator
  (params (Start :type Vector%20%28by%20ref%29) (Target :type Vector%20%28by%20ref%29) (DistanceFactor :type Float%20%28double-precision%29) (RotationOffset :type Float%20%28double-precision%29) (BezierWidth :type Float%20%28double-precision%29))
  (bind _returnvalue (Math|Rotator|FindLookatRotation Start Target))
  (bind (_roll _pitch _yaw) (Math|Rotator|BreakRotator _returnvalue))
  (return (+ (* (Math|Vector|GetRightVector (Math|Rotator|MakeRotator (+ _roll RotationOffset) _pitch _yaw)) BezierWidth) (+ (* (Math|Vector|GetForwardVector _returnvalue) (* (Math|Vector|Distance(Vector) Start Target) DistanceFactor)) (Variables|Default|GetLocationStart)))))